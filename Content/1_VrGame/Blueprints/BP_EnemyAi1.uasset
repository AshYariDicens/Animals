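; Enemy AI character that chases the player and attacks with a sword, and gets knocked down when its capsule is overlapped.
; PawnSensing sightings trigger an AI move to the player, followed by an attack montage and punch sound on arrival.
; Capsule overlaps block new chases and play fall and get-up montages, using montage-length delays and flags for timing.
; The sight flag is never cleared, as its reset logic is unconnected.
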(event `self.ReceiveBeginPlay`)

(event `self.ReceiveTick`
  (params (DeltaSeconds :type "Float (single-precision)")))

(event `self.PawnSensing.OnSeePawn`
  (params (Pawn :type "Pawn Object Reference"))
  (set `self.IsSeeingPlayer?` true)
  (`self.FollowPlayer`))

(event `FollowPlayer`
  (set `self.CanAttack?` true)
  (if (and (`self.IsSeeingPlayer?`) (`self.NotOverlapping?`))
    (`|AIMoveTo` self (0.0 0.0 0.0) (`GameplayStatics.GetPlayerPawn` 0) 110.0
      (:`OnSuccess`
        (if (`self.CanAttack?`)
          (set `self.CanAttack?` false)
          (set `self.NotOverlapping?` true)
          (`GameplayStatics.PlaySound2D` "/Game/1_VrGame/Sonido/Punch_04.Punch_04" 1.0 1.0 0.0 null null)
          (bind _returnvalue (`self.PlayAnimMontage` "/Game/Personajes/Cow/Cow_animations/AM_AtaqueEspada.AM_AtaqueEspada"))
          (`KismetSystemLibrary.Delay` _returnvalue)
          (set `self.CanAttack?` true))))
    (else
      (`self.Falling`)
      (`MovementComponent.StopMovementImmediately` (`self.CharacterMovement`)))))

(event `self.CapsuleComponent.OnComponentBeginOverlap`
  (params (OverlappedComponent :type "PrimitiveComponent Object Reference") (OtherActor :type "Actor Object Reference") (OtherComp :type "PrimitiveComponent Object Reference") (OtherBodyIndex :type Integer) (bFromSweep :type Boolean) (SweepResult :type "HitResult Structure (by ref)"))
  (set `self.NotOverlapping?` false)
  (`self.Falling`)
  (`KismetSystemLibrary.Delay` (stale `Falling` _returnvalue))
  (`KismetSystemLibrary.Delay` (stale `Falling` _returnvalue_2))
  (set `self.NotOverlapping?` true))

(event `Falling`
  (if (`self.CanFall?`)
    (set `self.CanFall?` false)
    (`GameplayStatics.PlaySound2D` "/Game/1_VrGame/Sonido/Punch_03.Punch_03" 1.0 1.0 0.0 null null)
    (bind _returnvalue (`self.PlayAnimMontage` "/Game/Personajes/Cow/Cow_animations/AM_Derribar.AM_Derribar"))
    (`KismetSystemLibrary.Delay` _returnvalue)
    (bind _returnvalue_2 (`self.PlayAnimMontage` "/Game/Personajes/Cat_Default/Animations/AM_LevantarseBocaArriba.AM_LevantarseBocaArriba"))
    (`KismetSystemLibrary.Delay` _returnvalue_2)
    (set `self.CanFall?` true)))

(fn `UserConstructionScript`)